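; Physics-driven flying wyrm pawn that the player flies by flapping front and back wing pairs through Enhanced Input.
; Each flap pushes the body upward and briefly fires that pair's thruster while tilting the wings.
; Repeatedly flapping one pair without the other also fires a pitch thruster.
; Mouse X direction rolls and yaws the body, while stabilize eases out roll and kills spin, and brake gradually decays velocity.
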(event `self.ReceiveBeginPlay`
  (set `self.thrusterActiveLength` 0.5)
  (set `self.consistentUpwardFlapForce` (0.0 0.0 15000000.0))
  (set `self.consecutiveFrontFlaps` 0)
  (set `self.consecutiveBackFlaps` 0))

(event `EnhancedInput|/Game/SkyRacePrototype/IA_FlapFrontWings`
  (params (ActionValue :type Boolean) (ElapsedSeconds :type "Float (double-precision)") (TriggeredSeconds :type "Float (double-precision)") (InputAction :type "InputAction Object Reference" :default "/Game/SkyRacePrototype/IA_FlapFrontWings.IA_FlapFrontWings"))
  (:`Started`
    (set `self.consecutiveBackFlaps` 0)
    (bind _result (`/Engine/EditorBlueprintResources/StandardMacros.IncrementInt` (`self.consecutiveFrontFlaps`))
      (:`  `
        (if (>= _result 5)
          (`ActorComponent.Activate` (`self.IncreasePitchThruster`) false))
        (`PrimitiveComponent.AddForce` (`self.Body`) (`self.consistentUpwardFlapForce`) "None" false)
        (`ActorComponent.Activate` (`self.FrontWingsThruster`) false)
        (`SceneComponent.K2_SetRelativeRotation` (`self.FrontWings`) (struct :`Pitch` -10.0) false false)
        (`KismetSystemLibrary.Delay` (`self.thrusterActiveLength`))
        (`ActorComponent.Deactivate` (`self.FrontWingsThruster`) :!label _label)
        (`ActorComponent.Deactivate` (`self.IncreasePitchThruster`))
        (`SceneComponent.K2_SetRelativeRotation` :`self` (`self.FrontWings`)))))
  (:`Completed`
    (goto _label)))

(event `EnhancedInput|/Game/SkyRacePrototype/IA_FlapBackWings`
  (params (ActionValue :type Boolean) (ElapsedSeconds :type "Float (double-precision)") (TriggeredSeconds :type "Float (double-precision)") (InputAction :type "InputAction Object Reference" :default "/Game/SkyRacePrototype/IA_FlapBackWings.IA_FlapBackWings"))
  (:`Started`
    (set `self.consecutiveFrontFlaps` 0)
    (bind _result (`/Engine/EditorBlueprintResources/StandardMacros.IncrementInt` (`self.consecutiveBackFlaps`))
      (:`  `
        (if (>= _result 5)
          (`ActorComponent.Activate` (`self.DecreasePitchThruster`) false))
        (`PrimitiveComponent.AddForce` (`self.Body`) (`self.consistentUpwardFlapForce`) "None" false)
        (`ActorComponent.Activate` (`self.BackWingsThruster`) false)
        (`SceneComponent.K2_SetRelativeRotation` (`self.BackWings`) (struct :`Pitch` -10.0) false false)
        (`KismetSystemLibrary.Delay` (`self.thrusterActiveLength`))
        (`ActorComponent.Deactivate` (`self.BackWingsThruster`))
        (`ActorComponent.Deactivate` (`self.DecreasePitchThruster`))
        (`SceneComponent.K2_SetRelativeRotation` :`self` (`self.BackWings`))))))

(event `EnhancedInput|/Game/SkyRacePrototype/IA_Roll`
  (params (ActionValue :type Boolean) (ElapsedSeconds :type "Float (double-precision)") (TriggeredSeconds :type "Float (double-precision)") (InputAction :type "InputAction Object Reference" :default "/Game/SkyRacePrototype/IA_Roll.IA_Roll"))
  (:`Triggered`
    (bind _returnvalue (`WidgetLayoutLibrary.GetMousePositionOnPlatform`))
    (bind _x (`KismetMathLibrary.BreakVector2D` _returnvalue))
    (if (> _x (`self.prevMouseX`))
      (`SceneComponent.K2_AddRelativeRotation` (`self.Body`) (struct :`Yaw` 0.5 :`Roll` 1.0) false false)
      (else
        (`SceneComponent.K2_AddRelativeRotation` (`self.Body`) (struct :`Yaw` -0.5 :`Roll` -1.0) false false)))
    (set `self.prevMouseX` _x)))

(event `EnhancedInput|/Game/SkyRacePrototype/IA_Stabilize`
  (params (ActionValue :type Boolean) (ElapsedSeconds :type "Float (double-precision)") (TriggeredSeconds :type "Float (double-precision)") (InputAction :type "InputAction Object Reference" :default "/Game/SkyRacePrototype/IA_Stabilize.IA_Stabilize"))
  (bind _body (`self.Body`))
  (:`Triggered`
    (`SceneComponent.K2_SetWorldRotation` _body (`KismetMathLibrary.MakeRotator` (/ (.roll (`SceneComponent.K2_GetComponentRotation` _body)) 1.05) (.pitch (`SceneComponent.K2_GetComponentRotation` _body)) (.yaw (`SceneComponent.K2_GetComponentRotation` _body))) false false)
    (`PrimitiveComponent.SetPhysicsAngularVelocityInDegrees` (`self.Body`) (0.0 0.0 0.0) false "None")))

(event `EnhancedInput|/Game/SkyRacePrototype/IA_Brake`
  (params (ActionValue :type Boolean) (ElapsedSeconds :type "Float (double-precision)") (TriggeredSeconds :type "Float (double-precision)") (InputAction :type "InputAction Object Reference" :default "/Game/SkyRacePrototype/IA_Brake.IA_Brake"))
  (bind _body (`self.Body`))
  (:`Triggered`
    (bind _returnvalue (`PrimitiveComponent.GetPhysicsLinearVelocity` _body "None"))
    (`PrimitiveComponent.SetPhysicsLinearVelocity` _body (/ _returnvalue (1.01 1.01 1.01)) false "None")))

(fn `UserConstructionScript`)